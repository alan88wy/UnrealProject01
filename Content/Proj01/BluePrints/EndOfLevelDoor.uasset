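; End-of-level door actor that swings open once when the player triggers the use-object Enhanced Input action.
; BeginPlay enables input from player controller 0, so the action fires with no overlap or proximity check.
; A DoOnce, never reset, stores the starting rotation and plays a timeline whose value is subtracted from the whole actor's yaw.
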(event Input|EnhancedActionEvents|EnhancedInputActionIA_UseObject
  (params (ActionValue :type Boolean) (ElapsedSeconds :type Float%20%28double-precision%29) (TriggeredSeconds :type Float%20%28double-precision%29) (InputAction :type Input%20Action%20Object%20Reference :default "/Game/Proj01/BluePrints/IA_UseObject.IA_UseObject"))
  ;[1 1 1] Open Door
  (Utilities|FlowControl|DoOnce false
    (:Completed
      (bind _output_get (Variables|Default|SetInitialDoorRotation (Transformation|GetActorRotation)))
      (bind _opendoormovement (Timeline|OpenDoorTimeline Play)
        (:Update
          (Transformation|SetActorRotation (Math|Rotator|MakeRotator (.Roll (Math|Rotator|BreakRotator _output_get)) (.Pitch (Math|Rotator|BreakRotator _output_get)) (- (.Yaw (Math|Rotator|BreakRotator _output_get)) _opendoormovement))))))))

(event EventBeginPlay
  (Input|EnableInput (Game|GetPlayerController 0)))

(event Collision|EventActorBeginOverlap
  (params (OtherActor :type Actor%20Object%20Reference)))

(event EventTick
  (params (DeltaSeconds :type Float%20%28single-precision%29)))

(fn ConstructionScript)