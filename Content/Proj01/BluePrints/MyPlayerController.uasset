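; MyPlayerController is a player controller that routes Enhanced Input actions to the player's MyCharacter and toggles game pause.
; On BeginPlay it casts player character 0 to MyCharacter and caches the reference for the input events.
; Move input drives movement along the character's right and forward vectors, and jump calls the character's Jump.
; Look input applies only yaw, as the pitch node is never run.
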(event Input|EnhancedActionEvents|EnhancedInputActionIA_Jump
  (params (ActionValue :type Boolean) (ElapsedSeconds :type Float%20%28double-precision%29) (TriggeredSeconds :type Float%20%28double-precision%29) (InputAction :type Input%20Action%20Object%20Reference :default "/Game/Proj01/BluePrints/IA_Jump.IA_Jump"))
  ;[1 1 1] Character Jump
  (Character|Jump (Variables|Default|GetMyCharacter)))

(event Input|EnhancedActionEvents|EnhancedInputActionIA_Look
  (params (ActionValue :type Vector%202D%20Structure) (ElapsedSeconds :type Float%20%28double-precision%29) (TriggeredSeconds :type Float%20%28double-precision%29) (InputAction :type Input%20Action%20Object%20Reference :default "/Game/Proj01/BluePrints/IA_Look.IA_Look"))
  ;[1 1 1] Character Look Around
  (Pawn|Input|AddControllerYawInput (Variables|Default|GetMyCharacter) (.x ActionValue)))

(event Input|EnhancedActionEvents|EnhancedInputActionIA_Move
  (params (ActionValue :type Vector%202D%20Structure) (ElapsedSeconds :type Float%20%28double-precision%29) (TriggeredSeconds :type Float%20%28double-precision%29) (InputAction :type Input%20Action%20Object%20Reference :default "/Game/Proj01/BluePrints/IA_Move.IA_Move"))
  (bind _mycharacter (Variables|Default|GetMyCharacter))
  ;[1 1 1] Character Movement
  (Pawn|Input|AddMovementInput _mycharacter (Transformation|GetActorRightVector _mycharacter) (.x ActionValue) false)
  (Pawn|Input|AddMovementInput _mycharacter (Transformation|GetActorForwardVector _mycharacter) (.y ActionValue) false))

(event Input|EnhancedActionEvents|EnhancedInputActionIA_Pause
  (params (ActionValue :type Boolean) (ElapsedSeconds :type Float%20%28double-precision%29) (TriggeredSeconds :type Float%20%28double-precision%29) (InputAction :type Input%20Action%20Object%20Reference :default "/Game/Proj01/BluePrints/IA_Pause.IA_Pause"))
  ;[1 1 1] Pause Game
  (if (Game|IsGamePaused)
    (Game|SetGamePaused false)
    (else
      (Game|SetGamePaused true))))

(event EventBeginPlay
  (bind _asmy_character (Utilities|Casting|CastToMyCharacter (Game|GetPlayerCharacter 0)))
  (Variables|Default|SetMyCharacter _asmy_character))

(event EventTick
  (params (DeltaSeconds :type Float%20%28single-precision%29)))

(fn ConstructionScript)